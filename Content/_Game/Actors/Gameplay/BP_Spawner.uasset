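; Spawner actor that launches BP_Particle actors along its cone's up vector with sound and Niagara effects.
; HUD widget events, bound through the player state, trigger cooldown-limited manual spawns or toggle a looping-timer auto spawner, which disables manual spawning.
; A player-stats event can stop auto spawning.
; On BeginPlay it launches a dummy particle and builds a trajectory from spline meshes along a predicted projectile path.
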(event Custom|LevelSpawner
  ;[0.15 0.15 0.15 0.5] Particle Spawning
  (if (not (Variables|Default|GetisOnCooldown))
    (Variables|Default|SetisOnCooldown true)
    (bind _returnvalue (Game|SpawnActorfromClass (Variables|Default|GetParticle) (Math|Conversions|ToTransform(Vector) (Transformation|GetActorLocation)) "Undefined" "MultiplyWithRoot" 0 0))
    (bind _asbp_particle (Utilities|Casting|CastToBP_Particle _returnvalue))
    (Physics|AddImpulse (Variables|/Game/_Game/Actors/Gameplay/BP_Particle.BP_Particle_C|GetSphere _asbp_particle) (* (Math|Vector|GetUpVector (Variables|Default|GetCone)) 1e+03) "None" true)
    (Audio|PlaySound2D "/Game/Audio/SFX/SpawnParticle_Cue.SpawnParticle_Cue" 1.0 1.0 0.0 0 0)
    (Niagara|SpawnSystematLocation "/Game/VFX/NS_ParticleHit.NS_ParticleHit" (Transformation|GetActorLocation self))
    (if (Variables|Default|GetAutoSpawnOn)
      (Variables|Default|SetIsOnCooldown false)
      (else
        (Utilities|Time|SetTimerbyEvent (delegate Custom|ResetCooldown) (Variables|Default|GetSpawnParticleCooldownTime))))))

(event Custom|ResetCooldown
  ;[0.15 0.15 0.15 0.5] Particle Spawning
  (Variables|Default|SetisOnCooldown false))

(event Custom|StopAutoSpawner
  ;[0.15 0.15 0.15 0.5] Stop Auto Spawner
  (if (Variables|Default|GetAutoSpawnOn)
    (CallFunction|ToggleManualSpawner)))

(event Custom|ToggleManualSpawner
  ;[0.15 0.15 0.15 0.5] Toggle Manual Spawn
  (bind _output_get (Variables|/Script/UMG.Widget|SetbIsEnabled (Variables|/Game/_Game/UI/Gameplay/WBP_HUD.WBP_HUD_C|GetWBP_ParticleSpawner (Variables|/Game/_Game/Blueprints/PS_PlayerStats.PS_PlayerStats_C|GetGameHUD (stale EventBeginPlay _asps_player_stats))) (not (Class|Widget|GetIsEnabled (Variables|/Game/_Game/UI/Gameplay/WBP_HUD.WBP_HUD_C|GetWBP_ParticleSpawner (Variables|/Game/_Game/Blueprints/PS_PlayerStats.PS_PlayerStats_C|GetGameHUD (stale EventBeginPlay _asps_player_stats)))))))
  (if (not _output_get)
    (Variables|Default|SetAutoSpawnOn true)
    (Default|AutoSpawneron (Variables|/Game/_Game/UI/Gameplay/WBP_HUD.WBP_HUD_C|GetWBP_AutoSpawner (Variables|/Game/_Game/Blueprints/PS_PlayerStats.PS_PlayerStats_C|GetGameHUD (stale EventBeginPlay _asps_player_stats))))
    (Audio|PlaySound2D "/Game/Audio/SFX/AutoSpawn_Cue.AutoSpawn_Cue" 1.0 1.0 0.0 0 0)
    (bind _returnvalue (Utilities|Time|SetTimerbyEvent (delegate Custom|LevelSpawner) (+ (Variables|Default|GetSpawnParticleCooldownTime) 0.1) true))
    (Variables|Default|SetAutoSpawnTimer _returnvalue)
    (else
      (Default|AutoSpawnerOff (Variables|/Game/_Game/UI/Gameplay/WBP_HUD.WBP_HUD_C|GetWBP_AutoSpawner (Variables|/Game/_Game/Blueprints/PS_PlayerStats.PS_PlayerStats_C|GetGameHUD (stale EventBeginPlay _asps_player_stats))))
      (Audio|PlaySound2D "/Game/Audio/SFX/AutoSpawnOff_Cue.AutoSpawnOff_Cue" 1.0 1.0 0.0 0 0)
      (Variables|Default|SetAutoSpawnOn false)
      (Variables|Default|SetIsOnCooldown false)
      (Utilities|Time|ClearandInvalidateTimerbyHandle (Variables|Default|GetAutoSpawnTimer)))))

(event EventBeginPlay
  (bind _cone (Variables|Default|GetCone))
  (bind _returnvalue (Math|Vector|GetUpVector _cone))
  (bind _returnvalue_2 (* _returnvalue 1e+03))
  ;[0.15 0.15 0.15 0.5] Begin Play
  (Utilities|FlowControl|DelayUntilNextFrame)
  (Spline|ClearSplinePoints (Variables|Default|GetSpline) true)
  (bind _asps_player_stats (Utilities|Casting|CastToPS_PlayerStats (Game|GetPlayerState 0)))
  (Utilities|IsValid (Variables|/Game/_Game/Blueprints/PS_PlayerStats.PS_PlayerStats_C|GetGameHUD _asps_player_stats)
    (:Is%20Valid
      (EventDispatchers|BindEventtoStopAutoSpawer _asps_player_stats (delegate Custom|StopAutoSpawner))
      (EventDispatchers|BindEventtoSpawnParticle (Variables|/Game/_Game/UI/Gameplay/WBP_HUD.WBP_HUD_C|GetWBP_ParticleSpawner (Variables|/Game/_Game/Blueprints/PS_PlayerStats.PS_PlayerStats_C|GetGameHUD _asps_player_stats)) (delegate Custom|LevelSpawner))
      (EventDispatchers|BindEventtoDisableManualSpawner (Variables|/Game/_Game/UI/Gameplay/WBP_HUD.WBP_HUD_C|GetWBP_AutoSpawner (Variables|/Game/_Game/Blueprints/PS_PlayerStats.PS_PlayerStats_C|GetGameHUD _asps_player_stats)) (delegate Custom|ToggleManualSpawner))
      (Variables|Default|SetSpawnParticleCooldownTime (Variables|/Game/_Game/Blueprints/PDA_Stats.PDA_Stats_C|GetParticleSpawnCooldown (Variables|Default|GetPDA_Stats)))
      (Variables|Default|SetAutoSpawnOn false)
      ;[0.15 0.15 0.15 0.5] Create Trajectory of particles
      (bind _returnvalue_3 (Game|SpawnActorfromClass (Variables|Default|GetDummyParticle) (Math|Conversions|ToTransform(Vector) (Transformation|GetActorLocation)) "Undefined" "MultiplyWithRoot" 0 0))
      (bind _asbp_dummy_particle (Utilities|Casting|CastToBP_DummyParticle _returnvalue_3))
      (Physics|AddImpulse (Variables|/Game/_Game/Actors/Gameplay/BP_DummyParticle.BP_DummyParticle_C|GetSphere _asbp_dummy_particle) _returnvalue_2 "None" true)
      (bind _outpathpositions (Class|GameplayStatics|BlueprintPredictProjectilePathbyTraceChannel (Transformation|GetActorLocation _asbp_dummy_particle) _returnvalue_2 false 0.0 "ECC_WorldDynamic" false 0 "None"))
      (for (_array_element _array_index) _outpathpositions
        (Spline|AddSplinePoint (Variables|Default|GetSpline) _array_element "Local" true))
      (Spline|SetSplinePointType (Variables|Default|GetSpline) _array_index "CurveClamped" true)
      (for _index (range 0 (Spline|GetNumberOfSplinePoints (Variables|Default|GetSpline)))
        (bind _returnvalue_4 (AddComponent|AddSplineMeshComponent true))
        (Utilities|Array|Add (Variables|Default|GetTrag%20Spline%20Mesh) _returnvalue_4)
        (SplineMesh|SetStartandEnd _returnvalue_4 (.Location (Spline|GetLocationandTangentatSplinePoint (Variables|Default|GetSpline) _index "Local")) (.Tangent (Spline|GetLocationandTangentatSplinePoint (Variables|Default|GetSpline) _index "Local")) (.Location (Spline|GetLocationandTangentatSplinePoint (Variables|Default|GetSpline) (+ _index 1) "Local")) (.Tangent (Spline|GetLocationandTangentatSplinePoint (Variables|Default|GetSpline) (+ _index 1) "Local")) true :!class /Script/Engine.SplineMeshComponent)))
    (:Is%20Not%20Valid
      (Development|PrintString "HUD BROKEN"))))

(fn ConstructionScript)