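; BP_Particle is a physics sphere that produces energy and heat for the player when it collides with another particle, and is destroyed on hitting the ground.
; It takes yields and cooldown from a stats data asset and a unique ID from the game mode.
; Only the higher-ID particle of a colliding pair awards stats, subject to its cooldown.
; Push item bumpers and pull item overlaps apply velocity impulses along the item's up axis.
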(event OnComponentBeginOverlap(Sphere)
  (params (OverlappedComponent :type Primitive%20Component%20Object%20Reference) (OtherActor :type Actor%20Object%20Reference) (OtherComp :type Primitive%20Component%20Object%20Reference) (OtherBodyIndex :type Integer) (bFromSweep :type Boolean) (SweepResult :type Hit%20Result%20Structure%20%28by%20ref%29))
  ;[0.15 0.15 0.15 0.5] Overlap Pull Item
  (if (== (Utilities|GetClass OtherActor) "/Game/_Game/Actors/Gameplay/BP_PullItem.BP_PullItem_C")
    (bind _asbp_pull_item (Utilities|Casting|CastToBP_PullItem OtherActor))
    (Physics|AddImpulse (Variables|Default|GetSphere) (* (* (Math|Vector|GetUpVector (Variables|/Game/_Game/Actors/Gameplay/BP_PullItem.BP_PullItem_C|GetBox _asbp_pull_item)) -1) 1e+03) "None" true)))

(event Custom|ResetCooldown
  ;[0.15 0.15 0.15 0.5] On Hit
  ;;[0.15 0.15 0.15 0.5] Hit Particle
  (Variables|Default|SetonEnergyCooldown false))

(event EventBeginPlay
  (bind _pda_stats (Variables|PDA_Stats|GetPDA_Stats))
  ;[0.15 0.15 0.15 0.5] Begin Play
  (Variables|Default|SetProducedEnergy (Variables|/Game/_Game/Blueprints/PDA_Stats.PDA_Stats_C|GetBaseEnergyAdd _pda_stats))
  (Variables|Default|SetAddEnergyCooldownTime (Variables|/Game/_Game/Blueprints/PDA_Stats.PDA_Stats_C|GetParticleAddEnergyCooldown _pda_stats))
  (Variables|Default|SetProducedHeat (Variables|/Game/_Game/Blueprints/PDA_Stats.PDA_Stats_C|GetBaseHeatAdd _pda_stats))
  (bind _asgm_game_mode (Utilities|Casting|CastToGM_GameMode (Game|GetGameMode)))
  (Variables|Default|SetParticleID (Variables|/Game/_Game/Blueprints/GM_GameMode.GM_GameMode_C|GetNextParticleID _asgm_game_mode))
  (Math|Integer|IncrementInt (Variables|/Game/_Game/Blueprints/GM_GameMode.GM_GameMode_C|GetNextParticleID _asgm_game_mode)))

(event Collision|EventHit
  (params (MyComp :type Primitive%20Component%20Object%20Reference) (Other :type Actor%20Object%20Reference) (OtherComp :type Primitive%20Component%20Object%20Reference) (bSelfMoved :type Boolean) (HitLocation :type Vector :default "0, 0, 0") (HitNormal :type Vector :default "0, 0, 0") (NormalImpulse :type Vector :default "0, 0, 0") (Hit :type Hit%20Result%20Structure%20%28by%20ref%29))
  (bind _returnvalue (Utilities|GetClass Other))
  ;[0.15 0.15 0.15 0.5] On Hit
  (Niagara|SpawnSystematLocation "/Game/VFX/NS_ParticleHit.NS_ParticleHit" (Transformation|GetWorldLocation (Variables|Default|GetSphere)))
  ;;[0.15 0.15 0.15 0.5] Hit Ground
  (if (== _returnvalue "/Game/_Game/Actors/Gameplay/BP_Ground.BP_Ground_C")
    (Actor|DestroyActor)
    (else
      ;;[0.15 0.15 0.15 0.5] Hit Particle
      (if (== _returnvalue "BP_Particle_C")
        (bind _asbp_particle (Utilities|Casting|CastToBP_Particle Other))
        (if (< (Variables|BP_Particle_C|GetParticleID _asbp_particle) (Variables|Default|GetParticleID))
          (if (not (Variables|Default|GetonEnergyCooldown))
            (Variables|Default|SetonEnergyCooldown true)
            (Utilities|Time|SetTimerbyEvent (delegate Custom|ResetCooldown) (Variables|Default|GetAddEnergyCooldownTime))
            (bind _asps_player_stats (Utilities|Casting|CastToPS_PlayerStats (Game|GetPlayerState 0)))
            (Default|AddEnergy _asps_player_stats (Variables|Default|GetProducedEnergy))
            (Default|AddHeat _asps_player_stats (Variables|Default|GetProducedHeat))
            (Audio|PlaySound2D "/Game/Audio/SFX/AddEnergy_Cue.AddEnergy_Cue" 1.0 1.0 0.0 0 0)))
        (else
          ;;[0.15 0.15 0.15 0.5] Hit Push Item
          (if (== _returnvalue "/Game/_Game/Actors/Gameplay/BP_PushItem.BP_PushItem_C")
            (bind _asbp_push_item (Utilities|Casting|CastToBP_PushItem Other))
            (if (== (Variables|/Game/_Game/Actors/Gameplay/BP_PushItem.BP_PushItem_C|GetBumper _asbp_push_item) OtherComp)
              (Physics|AddImpulse (Variables|Default|GetSphere) (* (Math|Vector|GetUpVector (Variables|/Game/_Game/Actors/Gameplay/BP_PushItem.BP_PushItem_C|GetBox _asbp_push_item)) 1e+03) "None" true))))))))

(fn ConstructionScript)