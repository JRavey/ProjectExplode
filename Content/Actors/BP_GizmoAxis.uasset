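; Mouse-driven transform gizmo that moves and yaw-rotates BP_BaseItem objects along X, Y, Z and rotation handles.
; Right-click traces under the cursor and attaches the hit component to the Rotation handle, detaching the previous one.
; Left-click picks a handle; Tick moves the root by the cursor offset projected onto that axis, or rotates by mouse delta.
; Handles highlight yellow on hover.
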(event OnBeginCursorOver(X)
  (params (TouchedComponent :type Primitive%20Component%20Object%20Reference))
  ;[0.15 0.15 0.15 0.5] Highlight Material
  (Rendering|Material|SetMaterial (Variables|Default|GetX) 0 "/Game/Material/M_ArrowYellow.M_ArrowYellow")
  (Utilities|FlowControl|Gate true) ; enters at Open
)

(event OnBeginCursorOver(Y)
  (params (TouchedComponent :type Primitive%20Component%20Object%20Reference))
  ;[0.15 0.15 0.15 0.5] Highlight Material
  (Rendering|Material|SetMaterial (Variables|Default|GetY) 0 "/Game/Material/M_ArrowYellow.M_ArrowYellow")
  (Utilities|FlowControl|Gate true) ; enters at Open
)

(event OnBeginCursorOver(Z)
  (params (TouchedComponent :type Primitive%20Component%20Object%20Reference))
  ;[0.15 0.15 0.15 0.5] Highlight Material
  (Rendering|Material|SetMaterial (Variables|Default|GetZ) 0 "/Game/Material/M_ArrowYellow.M_ArrowYellow")
  (Utilities|FlowControl|Gate true) ; enters at Open
)

(event OnEndCursorOver(X)
  (params (TouchedComponent :type Primitive%20Component%20Object%20Reference))
  ;[0.15 0.15 0.15 0.5] Highlight Material
  (Rendering|Material|SetMaterial (Variables|Default|GetX) 0 "/Game/Material/M_ArrowRed.M_ArrowRed")
  (Utilities|FlowControl|Gate true) ; enters at Close
)

(event OnEndCursorOver(Y)
  (params (TouchedComponent :type Primitive%20Component%20Object%20Reference))
  ;[0.15 0.15 0.15 0.5] Highlight Material
  (Rendering|Material|SetMaterial (Variables|Default|GetY) 0 "/Game/Material/M_ArrowGreen.M_ArrowGreen")
  (Utilities|FlowControl|Gate true) ; enters at Close
)

(event OnEndCursorOver(Z)
  (params (TouchedComponent :type Primitive%20Component%20Object%20Reference))
  ;[0.15 0.15 0.15 0.5] Highlight Material
  (Rendering|Material|SetMaterial (Variables|Default|GetZ) 0 "/Game/Material/M_ArrowBlue.M_ArrowBlue")
  (Utilities|FlowControl|Gate true) ; enters at Close
)

(event OnBeginCursorOver(Rotation)
  (params (TouchedComponent :type Primitive%20Component%20Object%20Reference))
  ;[0.15 0.15 0.15 0.5] Highlight Material
  (Rendering|Material|SetMaterial (Variables|Default|GetRotation) 0 "/Game/Material/M_ArrowYellow.M_ArrowYellow")
  (Utilities|FlowControl|Gate true) ; enters at Open
)

(event OnEndCursorOver(Rotation)
  (params (TouchedComponent :type Primitive%20Component%20Object%20Reference))
  ;[0.15 0.15 0.15 0.5] Highlight Material
  (Rendering|Material|SetMaterial (Variables|Default|GetRotation) 0 "/Game/Material/M_Red.M_Red")
  (Utilities|FlowControl|Gate true) ; enters at Close
)

(event EventBeginPlay
  ;[0.15 0.15 0.15 0.5] Enable Input
  (Input|EnableInput (Game|GetPlayerController 0)))

(event EventTick
  (params (DeltaSeconds :type Float%20%28single-precision%29))
  (bind _returnvalue (Game|GetPlayerController 0))
  (bind (_worldlocation _worlddirection) (Game|Player|ConvertMouseLocationToWorldSpace _returnvalue))
  (switch Utilities|FlowControl|Switch|SwitchonAxisVariable (.membervar (Utilities|Struct|MakeDragged_Axis 0 (CallFunction|AxisComponent (Variables|Default|GetAxis%20Dragged))))
    (:NewEnumerator0
      ;[0.15 0.15 0.15 0.5] Movement
      (Utilities|IsValid (Variables|Default|GetAxis%20Dragged) :!label _label
        (:Is%20Valid
          (Transformation|AddRelativeLocation (Variables|Default|GetGizmo%20Root) (/ (Math|Vector|ProjectVectorontoVector (Math|Transform|InverseTransformLocation (Math|Conversions|ToTransform(Vector) (Variables|Default|GetDragLocation)) (+ _worldlocation (* _worlddirection (Variables|Default|GetDistanceToGrab)))) (Math|Vector|GetForwardVector (Variables|Default|GetAxis%20Dragged))) 3e+01) false false))))
    (:NewEnumerator1
      (goto _label))
    (:NewEnumerator2
      (goto _label))
    (:NewEnumerator3
      ;[0.15 0.15 0.15 0.5] Rotation
      (Utilities|IsValid (Variables|Default|GetAxis%20Dragged)
        (:Is%20Valid
          (Transformation|AddLocalRotation (Variables|Default|GetRotation) (Math|Rotator|MakeRotator 0.0 0.0 (* (.DeltaX (Class|PlayerController|GetInputMouseDelta (Game|GetPlayerController 0))) -1e+01)) false false))))))

(event Input|MouseEvents|LeftMouseButton
  (params (Key :type Key%20Structure :default "None"))
  (bind _returnvalue (Game|GetPlayerController 0))
  (bind (_worldlocation _worlddirection) (Game|Player|ConvertMouseLocationToWorldSpace _returnvalue))
  ;[0.15 0.15 0.15 0.5] Gizmo Axis On Click
  (:Pressed
    (bind _outhit (Collision|LineTraceByChannel _worldlocation (+ _worldlocation (* _worlddirection 1e+04)) "TraceTypeQuery1" true 0 "ForDuration" false))
    (Variables|Default|SetDistanceToGrab (.Distance (Collision|BreakHitResult _outhit)))
    (switch Utilities|FlowControl|Switch|SwitchonAxisVariable (.membervar (Utilities|Struct|MakeDragged_Axis 0 (CallFunction|AxisComponent (.HitComponent (Collision|BreakHitResult _outhit)))))
      (:NewEnumerator0
        _)
      (:NewEnumerator1
        _)
      (:NewEnumerator2
        _))
    (Variables|Default|SetDragLocation (Math|Transform|InverseTransformLocation (Math|Conversions|ToTransform(Vector) (Math|Conversions|ToVector(Float) (Class|GameplayStatics|GetWorldOriginLocation))) (.Location (Collision|BreakHitResult _outhit)))))
  (:Released
    (Variables|Default|SetAxis%20Dragged 0)))

(event Input|MouseEvents|RightMouseButton
  (params (Key :type Key%20Structure :default "None"))
  (bind _returnvalue (Game|GetPlayerController 0))
  (bind (_worldlocation _worlddirection) (Game|Player|ConvertMouseLocationToWorldSpace _returnvalue))
  ;[0.15 0.15 0.15 0.5] Right Click to add Gizmo to actor
  (:Pressed
    (Utilities|IsValid (Variables|Default|GetLast%20Hit%20Component)
      (:Is%20Valid
        (Transformation|DetachFromComponent (Variables|Default|GetLast%20Hit%20Component) "KeepWorld" "KeepWorld" "KeepRelative" true))
      (:Is%20Not%20Valid
        _))
    (Rendering|SetVisibility (Variables|Default|GetGizmo%20Root) false true)
    (bind _outhit (Collision|LineTraceByChannel _worldlocation (+ _worldlocation (* _worlddirection 1e+04)) "TraceTypeQuery1" true 0 "ForDuration" false))
    (Utilities|IsValid (.HitComponent (Collision|BreakHitResult _outhit))
      (:Is%20Valid
        (if (Utilities|ClassIsChildOf (Utilities|GetClass (.HitActor (Collision|BreakHitResult _outhit))) "/Game/Actors/BP_BaseItem.BP_BaseItem_C")
          (Variables|Default|SetLast%20Hit%20Component (.HitComponent (Collision|BreakHitResult _outhit)))
          (Rendering|SetVisibility (Variables|Default|GetGizmo%20Root) true true)
          (Transformation|SetWorldLocation (Variables|Default|GetGizmo%20Root) (Math|Vector|MakeVector (.x (Transformation|GetWorldLocation (Variables|Default|GetLast%20Hit%20Component))) (.y (Transformation|GetWorldLocation (Variables|Default|GetLast%20Hit%20Component))) (.z (Transformation|GetWorldLocation (Variables|Default|GetLast%20Hit%20Component)))) false false)
          (Transformation|AttachComponentToComponent (Variables|Default|GetLast%20Hit%20Component) (Variables|Default|GetRotation) "None" "KeepWorld" "KeepWorld" "KeepRelative" true))))))

(fn ConstructionScript)

(fn AxisComponent
  (params (Axis_component :type Primitive%20Component%20Object%20Reference))
  (Variables|Default|SetAxis%20Dragged Axis_component)
  (if (== (Variables|Default|GetAxis%20Dragged) (Variables|Default|GetX))
    (return "NewEnumerator0")
    (elif (== (Variables|Default|GetAxis%20Dragged) (Variables|Default|GetY))
      (return "NewEnumerator1")
      (elif (== (Variables|Default|GetAxis%20Dragged) (Variables|Default|GetZ))
        (return "NewEnumerator2")
        (elif (== (Variables|Default|GetAxis%20Dragged) (Variables|Default|GetRotation))
          (return "NewEnumerator3")
          (else
            (Variables|Default|SetAxis%20Dragged 0)))))))