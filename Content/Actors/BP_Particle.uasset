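; BP_Particle is an actor that produces energy for the player when it collides with other particles.
; On hit, it destroys itself against BP_Ground and adds ProducedEnergy to player 0's PS_PlayerStats against another BP_Particle.
; A short timer-reset cooldown throttles energy gain.
; The cooldown flag is set before the particle cast, so hitting anything else first leaves it set without a reset timer.
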(event Custom|ResetEnergyCooldown
  ;[0.15 0.15 0.15 0.5] Add Energy
  (Variables|Default|SetisOnEnergyCooldown false))

(event Collision|EventHit
  (params (MyComp :type Primitive%20Component%20Object%20Reference) (Other :type Actor%20Object%20Reference) (OtherComp :type Primitive%20Component%20Object%20Reference) (bSelfMoved :type Boolean) (HitLocation :type Vector :default "0, 0, 0") (HitNormal :type Vector :default "0, 0, 0") (NormalImpulse :type Vector :default "0, 0, 0") (Hit :type Hit%20Result%20Structure%20%28by%20ref%29))
  (Utilities|FlowControl|Sequence
    (:then_0
      ;[0.15 0.15 0.15 0.5] Destory Actor
      (Utilities|Casting|CastToBP_Ground Other)
      (Actor|DestroyActor))
    (:then_1
      ;[0.15 0.15 0.15 0.5] Add Energy
      (if (not (Variables|Default|GetisOnEnergyCooldown))
        (Variables|Default|SetisOnEnergyCooldown true)
        (Utilities|Casting|CastToBP_Particle Other)
        (bind _asps_player_stats (Utilities|Casting|CastToPS_PlayerStats (Game|GetPlayerState 0)))
        (Default|AddEnergy _asps_player_stats (Variables|Default|GetProducedEnergy))
        (Utilities|Time|SetTimerbyEvent (delegate Custom|ResetEnergyCooldown) 0.35)))))

(fn ConstructionScript)